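; Player controller for a platformer that handles respawning, camera shakes, the crosshair and the pause menu.
; On UnPossess it asks BP_GameModeBase to respawn it, while Server_Respawn spawns and possesses a new BP_PlayerBase after a short delay.
; It adds the crosshair on BeginPlay, and the Menu input opens a UI-only pause menu, showing the cursor for non-gamepad keys.
; Camera shake events play shakes client-side, and PlatformerControllerRef returns the controller itself.
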(event `Client_CameraShake`
  (params (Shake :type "CameraShakeBase Class Reference"))
  (`self.ClientStartCameraShake` Shake))

(event `/Game/Assets/Blueprints/Interfaces/INT_Platformer_Controller.CameraShake`
  (params (CameraShake :type "MatineeCameraShake Class Reference"))
  (`self.Client_CameraShake` CameraShake))

(event `self.ReceiveBeginPlay`
  (bind _returnvalue (`|CreateWidget` "/Game/Assets/UI/W_Crosshair.W_Crosshair_C"))
  (`UserWidget.AddToViewport` _returnvalue 0))

(event `Server_Respawn`
  (params (SpawnTransform :type "Transform Structure"))
  ;[0 0 0 1 32] Server Respawn logic
  (bind _returnvalue (`|SpawnActorFromClass` "/Game/Assets/Blueprints/BP_PlayerBase.BP_PlayerBase_C" SpawnTransform "Undefined" "OverrideRootScale" null false null))
  (`KismetSystemLibrary.Delay` 0.1)
  (`self.Possess` _returnvalue))

(event `self.ReceiveUnPossess`
  (params (UnpossessedPawn :type "Pawn Object Reference"))
  ;[0 0 0 1 32] Respawn when the character dies to the world kill zone
  (bind _asbp_game_mode_base (cast `/Game/Assets/Blueprints/BP_GameModeBase` (`GameplayStatics.GetGameMode`)))
  (`/Game/Assets/Blueprints/BP_GameModeBase.Respawn` _asbp_game_mode_base self))

(event `InputAction|Menu`
  (params (Key :type "Key Structure"))
  ;[0 0 0 1 32] Pause Menu
  (:`Pressed`
    (if true
      (bind _returnvalue (`|CreateWidget` "/Game/Assets/UI/W_PauseMenu.W_PauseMenu_C"))
      (bind _output_get (set `self.PauseMenu` _returnvalue))
      (`UserWidget.AddToViewport` (`self.PauseMenu`) 0)
      (`UserWidget.AddToViewport` _output_get 0)
      (`WidgetBlueprintLibrary.SetInputMode_UIOnlyEx` self (`self.PauseMenu`))
      (if (`KismetInputLibrary.Key_IsGamepadKey` Key)
        (`KismetSystemLibrary.Delay` 0.2)
        (else
          (set `self.bShowMouseCursor` true))))))

(fn `PlatformerControllerRef`
  (returns (PlatformerControllerRef :type "/Game/Assets/Blueprints/BP_PlatformerController Object Reference"))
  (return self))

(fn `UserConstructionScript`)