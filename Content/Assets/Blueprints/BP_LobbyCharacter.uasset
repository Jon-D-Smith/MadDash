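; BP_LobbyCharacter is the lobby character that brings up the main menu when play begins.
; BeginPlay creates the W_MainMenu widget for the first player controller, adds it to the viewport, shows the cursor and sets Game and UI input focused on the menu.
; When the Steam online subsystem is present, it waits briefly, then passes the player's online nickname to the menu as the player name.
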(event `self.ReceiveBeginPlay`
  (bind _returnvalue (`|CreateWidget` "/Game/Assets/UI/W_MainMenu.W_MainMenu_C" (`GameplayStatics.GetPlayerController` 0)))
  (set `self.MainMenu` _returnvalue)
  (`UserWidget.AddToViewport` _returnvalue 0)
  (bind _returnvalue_2 (`Widget.GetOwningPlayer` _returnvalue))
  (set `PlayerController.bShowMouseCursor` true _returnvalue_2)
  (`WidgetBlueprintLibrary.SetInputMode_GameAndUIEx` _returnvalue_2 _returnvalue)
  (if (`AdvancedSessionsLibrary.HasOnlineSubsystem` "STEAM")
    (`KismetSystemLibrary.Delay` 0.2)
    (`/Game/Assets/UI/W_MainMenu.SetPlayerName` (`self.MainMenu`) (`KismetTextLibrary.Conv_StringToText` (`AdvancedIdentityLibrary.GetPlayerNickname` (`AdvancedSessionsLibrary.GetUniqueNetID` (`GameplayStatics.GetPlayerController` 0)))))))

(fn `UserConstructionScript`)