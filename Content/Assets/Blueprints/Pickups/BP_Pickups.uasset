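; Pickup actor, apparently a base for weapon pickups, that offers itself to players who walk into its sphere.
; On the server, overlap by a Player-tagged actor waits 0.2 seconds, then passes the pickup via SetPickupMessage; end overlap does nothing.
; It exposes weapon type and self getters, plus events to disable collision and destroy itself.
; FireWeapon forwards to a server fire event, left empty here for overriding.
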(event `Server_FireWeapon`
  ;[0 0 0 1 32] Overridden Events
)

(event `/Game/Assets/Blueprints/Pickups/INT_Pickup.DisableCollision`
  ;[0 0 0 1 32] Disable Collision
  (`PrimitiveComponent.SetCollisionEnabled` (`self.Sphere`) "NoCollision"))

(event `/Game/Assets/Blueprints/Pickups/INT_Pickup.FireWeapon`
  ;[0 0 0 1 32] Overridden Events
  (`self.Server_FireWeapon`))

(event `Server_RemovePickupFromWorld`
  ;[0 0 0 1 32] Delete pickup from the world
  (`self.K2_DestroyActor`))

(event `self.Sphere.OnComponentBeginOverlap`
  (params (OverlappedComponent :type "PrimitiveComponent Object Reference") (OtherActor :type "Actor Object Reference") (OtherComp :type "PrimitiveComponent Object Reference") (OtherBodyIndex :type Integer) (bFromSweep :type Boolean) (SweepResult :type "HitResult Structure (by ref)"))
  ;[0 0 0 1 32] Set Pickup
  (`/Engine/EditorBlueprintResources/ActorMacros.Switch Has Authority`
    (:`Authority`
      (if (`self.ActorHasTag` OtherActor "Player")
        (`KismetSystemLibrary.Delay` 0.2)
        (message `/Game/Assets/Blueprints/Interfaces/INT_PlatformerCharacter.SetPickup` OtherActor self)))))

(event `self.Sphere.OnComponentEndOverlap`
  (params (OverlappedComponent :type "PrimitiveComponent Object Reference") (OtherActor :type "Actor Object Reference") (OtherComp :type "PrimitiveComponent Object Reference") (OtherBodyIndex :type Integer))
  (`/Engine/EditorBlueprintResources/ActorMacros.Switch Has Authority`))

(fn `GetWeaponType`
  (returns (WeaponType :type "/Game/Assets/Blueprints/Pickups/Weapons/E_WeaponType Enum"))
  (return (`self.WeaponType`)))

(fn `PickupRef`
  (returns (PickupRef :type "/Game/Assets/Blueprints/Pickups/BP_Pickups Object Reference"))
  (return self))

(fn `UserConstructionScript`)