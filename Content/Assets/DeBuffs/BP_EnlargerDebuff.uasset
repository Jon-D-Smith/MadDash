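; Pickup debuff actor that doubles the scale of a platformer character touching its box, then restores normal size after a cooldown.
; Begin overlap destroys the box and mesh and scales the character through INT_PlatformerCharacter.
; End overlap waits for Cooldown, sets scale to one and destroys the actor.
; ServerGrow and ServerReset repeat this logic, intended for server replication, while PowerupFunction only prints the player's name.
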(event `self.Box.OnComponentBeginOverlap`
  (params (OverlappedComponent :type "PrimitiveComponent Object Reference") (OtherActor :type "Actor Object Reference") (OtherComp :type "PrimitiveComponent Object Reference") (OtherBodyIndex :type Integer) (bFromSweep :type Boolean) (SweepResult :type "HitResult Structure (by ref)"))
  ;[0 0 0 1 32] Grow double in size
  (`self.ServerGrow`)
  (bind _asint_platformer_character (cast `/Game/Assets/Blueprints/Interfaces/INT_PlatformerCharacter` OtherActor))
  (`ActorComponent.K2_DestroyComponent` (`self.Box`))
  (`ActorComponent.K2_DestroyComponent` (`self.StaticMesh`))
  (bind _platformerchar (`/Game/Assets/Blueprints/Interfaces/INT_PlatformerCharacter.PlatformerCharRef` _asint_platformer_character))
  (`self.SetActorRelativeScale3D` _platformerchar (* (`self.GetActorRelativeScale3D` _platformerchar) 2.0)))

(event `self.Box.OnComponentEndOverlap`
  (params (OverlappedComponent :type "PrimitiveComponent Object Reference") (OtherActor :type "Actor Object Reference") (OtherComp :type "PrimitiveComponent Object Reference") (OtherBodyIndex :type Integer))
  ;[0 0 0 1 32] Return to Normal Size
  (`self.ServerReset`)
  (`KismetSystemLibrary.Delay` (`self.Cooldown`))
  (bind _asint_platformer_character (cast `/Game/Assets/Blueprints/Interfaces/INT_PlatformerCharacter` OtherActor))
  (bind _platformerchar (`/Game/Assets/Blueprints/Interfaces/INT_PlatformerCharacter.PlatformerCharRef` _asint_platformer_character))
  (`self.SetActorRelativeScale3D` _platformerchar (1.0 1.0 1.0))
  (`self.K2_DestroyActor`))

(event `ServerGrow`
  ;[0 0 0 1 32] Replicate growth/shrink to server
  (bind _asint_platformer_character (cast `/Game/Assets/Blueprints/Interfaces/INT_PlatformerCharacter` (`self.Other Actor`)))
  (`ActorComponent.K2_DestroyComponent` (`self.Box`))
  (`ActorComponent.K2_DestroyComponent` (`self.StaticMesh`))
  (bind _platformerchar (`/Game/Assets/Blueprints/Interfaces/INT_PlatformerCharacter.PlatformerCharRef` _asint_platformer_character))
  (`self.SetActorRelativeScale3D` _platformerchar (* (`self.GetActorRelativeScale3D` _platformerchar) 2.0)))

(event `ServerReset`
  ;[0 0 0 1 32] Replicate growth/shrink to server
  (`KismetSystemLibrary.Delay` (`self.Cooldown`))
  (bind _asint_platformer_character (cast `/Game/Assets/Blueprints/Interfaces/INT_PlatformerCharacter` (`self.Other Actor`)))
  (bind _platformerchar (`/Game/Assets/Blueprints/Interfaces/INT_PlatformerCharacter.PlatformerCharRef` _asint_platformer_character))
  (`self.SetActorRelativeScale3D` _platformerchar (1.0 1.0 1.0))
  (`self.K2_DestroyActor`))

(event `/Game/Assets/Blueprints/Interfaces/INT_Powerup.PowerupFunction`
  (params (PlayerReference :type "Actor Object Reference"))
  (`KismetSystemLibrary.PrintString` (`KismetSystemLibrary.GetDisplayName` PlayerReference)))

(fn `UserConstructionScript`)