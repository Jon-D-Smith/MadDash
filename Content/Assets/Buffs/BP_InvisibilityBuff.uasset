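; Invisibility buff pickup that temporarily turns a platformer character's mesh to glass.
; Box overlap removes the box and visible mesh, then swaps the character's material via the INT_PlatformerCharacter interface.
; End overlap waits ten seconds, applies a flat grey material and destroys the actor.
; ServerInvis and ServerResetVisibility duplicate this logic for the server, while the graph's shrink and size comments don't match the behavior.
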(event `self.Box.OnComponentBeginOverlap`
  (params (OverlappedComponent :type "PrimitiveComponent Object Reference") (OtherActor :type "Actor Object Reference") (OtherComp :type "PrimitiveComponent Object Reference") (OtherBodyIndex :type Integer) (bFromSweep :type Boolean) (SweepResult :type "HitResult Structure (by ref)"))
  ;[0 0 0 1 32] Shrink half in size
  (`self.ServerInvis`)
  (bind _asint_platformer_character (cast `/Game/Assets/Blueprints/Interfaces/INT_PlatformerCharacter` OtherActor))
  (`ActorComponent.K2_DestroyComponent` (`self.Box`))
  (`ActorComponent.K2_DestroyComponent` (`self.StaticMesh`))
  (bind _platformerchar (`/Game/Assets/Blueprints/Interfaces/INT_PlatformerCharacter.PlatformerCharRef` _asint_platformer_character))
  (`PrimitiveComponent.SetMaterial` (`Character.Mesh` _platformerchar) 0 "/Game/StarterContent/Materials/M_Glass.M_Glass"))

(event `self.Box.OnComponentEndOverlap`
  (params (OverlappedComponent :type "PrimitiveComponent Object Reference") (OtherActor :type "Actor Object Reference") (OtherComp :type "PrimitiveComponent Object Reference") (OtherBodyIndex :type Integer))
  ;[0 0 0 1 32] Return to Normal Size
  (`self.ServerResetVisibility`)
  (`KismetSystemLibrary.Delay` 10.0)
  (bind _asint_platformer_character (cast `/Game/Assets/Blueprints/Interfaces/INT_PlatformerCharacter` OtherActor))
  (bind _platformerchar (`/Game/Assets/Blueprints/Interfaces/INT_PlatformerCharacter.PlatformerCharRef` _asint_platformer_character))
  (`PrimitiveComponent.SetMaterial` (`Character.Mesh` _platformerchar) 0 "/Game/Assets/Materials/M_FlatGreyLight_Inst.M_FlatGreyLight_Inst")
  (`self.K2_DestroyActor`))

(event `ServerInvis`
  ;[0 0 0 1 32] Replicate growth/shrink to server
  (bind _asint_platformer_character (cast `/Game/Assets/Blueprints/Interfaces/INT_PlatformerCharacter` (`self.Other Actor`)))
  (`ActorComponent.K2_DestroyComponent` (`self.Box`))
  (`ActorComponent.K2_DestroyComponent` (`self.StaticMesh`))
  (bind _platformerchar (`/Game/Assets/Blueprints/Interfaces/INT_PlatformerCharacter.PlatformerCharRef` _asint_platformer_character))
  (`PrimitiveComponent.SetMaterial` (`Character.Mesh` _platformerchar) 0 "/Game/StarterContent/Materials/M_Glass.M_Glass"))

(event `ServerResetVisibility`
  ;[0 0 0 1 32] Replicate growth/shrink to server
  (`KismetSystemLibrary.Delay` 10.0)
  (bind _asint_platformer_character (cast `/Game/Assets/Blueprints/Interfaces/INT_PlatformerCharacter` (`self.Other Actor`)))
  (bind _platformerchar (`/Game/Assets/Blueprints/Interfaces/INT_PlatformerCharacter.PlatformerCharRef` _asint_platformer_character))
  (`PrimitiveComponent.SetMaterial` (`Character.Mesh` _platformerchar) 0 "/Game/Assets/Materials/M_FlatGreyLight_Inst.M_FlatGreyLight_Inst")
  (`self.K2_DestroyActor`))

(fn `UserConstructionScript`)