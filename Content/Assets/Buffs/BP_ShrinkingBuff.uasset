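; Pickup buff that halves a platformer character's scale and capsule height when it overlaps the box.
; Begin overlap removes the box and mesh and resizes the character through the INT_PlatformerCharacter interface.
; End overlap restores default scale and capsule height after a ten-second delay, then destroys the actor.
; ServerShrink and ServerResetSize repeat this logic for replication, though ServerShrink doubles scale instead of halving it.
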(event `self.Box.OnComponentBeginOverlap`
  (params (OverlappedComponent :type "PrimitiveComponent Object Reference") (OtherActor :type "Actor Object Reference") (OtherComp :type "PrimitiveComponent Object Reference") (OtherBodyIndex :type Integer) (bFromSweep :type Boolean) (SweepResult :type "HitResult Structure (by ref)"))
  ;[0 0 0 1 32] Shrink half in size
  (`self.ServerShrink`)
  (bind _asint_platformer_character (cast `/Game/Assets/Blueprints/Interfaces/INT_PlatformerCharacter` OtherActor))
  (`ActorComponent.K2_DestroyComponent` (`self.Box`))
  (`ActorComponent.K2_DestroyComponent` (`self.StaticMesh`))
  (bind _platformerchar (`/Game/Assets/Blueprints/Interfaces/INT_PlatformerCharacter.PlatformerCharRef` _asint_platformer_character))
  (`self.SetActorRelativeScale3D` _platformerchar (* (`self.GetActorRelativeScale3D` _platformerchar) 0.5))
  (set `/Game/Assets/Blueprints/BP_PlayerBase.CapsuleHeight` (/ (`/Game/Assets/Blueprints/BP_PlayerBase.CapsuleHeight` _platformerchar) 2.0) _platformerchar))

(event `self.Box.OnComponentEndOverlap`
  (params (OverlappedComponent :type "PrimitiveComponent Object Reference") (OtherActor :type "Actor Object Reference") (OtherComp :type "PrimitiveComponent Object Reference") (OtherBodyIndex :type Integer))
  ;[0 0 0 1 32] Return to Normal Size
  (`self.ServerResetSize`)
  (`KismetSystemLibrary.Delay` 10.0)
  (bind _asint_platformer_character (cast `/Game/Assets/Blueprints/Interfaces/INT_PlatformerCharacter` OtherActor))
  (bind _platformerchar (`/Game/Assets/Blueprints/Interfaces/INT_PlatformerCharacter.PlatformerCharRef` _asint_platformer_character))
  (set `/Game/Assets/Blueprints/BP_PlayerBase.CapsuleHeight` 70.0 _platformerchar)
  (`self.SetActorRelativeScale3D` _platformerchar (1.0 1.0 1.0))
  (`self.K2_DestroyActor`))

(event `ServerShrink`
  ;[0 0 0 1 32] Replicate growth/shrink to server
  (bind _asint_platformer_character (cast `/Game/Assets/Blueprints/Interfaces/INT_PlatformerCharacter` (`self.Other Actor`)))
  (`ActorComponent.K2_DestroyComponent` (`self.Box`))
  (`ActorComponent.K2_DestroyComponent` (`self.StaticMesh`))
  (bind _platformerchar (`/Game/Assets/Blueprints/Interfaces/INT_PlatformerCharacter.PlatformerCharRef` _asint_platformer_character))
  (`self.SetActorRelativeScale3D` _platformerchar (* (`self.GetActorRelativeScale3D` _platformerchar) 2.0))
  (set `/Game/Assets/Blueprints/BP_PlayerBase.CapsuleHeight` (/ (`/Game/Assets/Blueprints/BP_PlayerBase.CapsuleHeight` _platformerchar) 2.0) _platformerchar))

(event `ServerResetSize`
  ;[0 0 0 1 32] Replicate growth/shrink to server
  (`KismetSystemLibrary.Delay` 10.0)
  (bind _asint_platformer_character (cast `/Game/Assets/Blueprints/Interfaces/INT_PlatformerCharacter` (`self.Other Actor`)))
  (bind _platformerchar (`/Game/Assets/Blueprints/Interfaces/INT_PlatformerCharacter.PlatformerCharRef` _asint_platformer_character))
  (`self.SetActorRelativeScale3D` _platformerchar (1.0 1.0 1.0))
  (set `/Game/Assets/Blueprints/BP_PlayerBase.CapsuleHeight` 70.0 _platformerchar)
  (`self.K2_DestroyActor`))

(fn `UserConstructionScript`)